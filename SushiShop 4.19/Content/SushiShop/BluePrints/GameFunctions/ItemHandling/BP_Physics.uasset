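; Physics-driven skeletal mesh item that can be picked up and dropped through Pickup and Drop events.
; Pickup stops simulation, attaches the root to the given component, then re-enables physics on bodies below an anchor bone, excluding that bone.
; Drop simulates the whole mesh again and detaches it.
; The anchor bone is the physics asset body closest to the mesh component's world location.
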(event EventBeginPlay)

(event Collision|EventActorBeginOverlap
  (params (OtherActor :type Actor%20Object%20Reference)))

(event EventPickup
  (params (Attach%20TO :type Scene%20Component%20Object%20Reference))
  ;[1 1 1] Open Class Settings and add the Pickup Actor Interface
  (Physics|SetSimulatePhysics (Variables|SkeletalMeshActor|GetSkeletalMeshComponent) false)
  (Transformation|AttachComponentToComponent (VehicleSound|GetRootComponent) Attach%20TO "None" "KeepWorld" "KeepWorld" "KeepWorld" false)
  (CallFunction|SetSimulateBelowBone))

(event EventDrop
  ;[1 1 1] Open Class Settings and add the Pickup Actor Interface
  (CallFunction|SetSimulateAll)
  (Physics|SetSimulatePhysics (Variables|SkeletalMeshActor|GetSkeletalMeshComponent) true)
  (Transformation|DetachFromActor "KeepWorld" "KeepWorld" "KeepWorld"))

(event EventTick
  (params (DeltaSeconds :type Float%20%28single-precision%29)))

(fn ConstructionScript)

(fn SetSimulateBelowBone
  (bind _skeletalmeshcomponent (Variables|SkeletalMeshActor|GetSkeletalMeshComponent))
  (Class|SkeletalMeshComponent|SetAllBodiesBelowSimulatePhysics (Variables|SkeletalMeshActor|GetSkeletalMeshComponent) (Utilities|Name|MakeLiteralName (.BoneName (Class|SkeletalMeshComponent|GetClosestPointonPhysicsAsset _skeletalmeshcomponent (Transformation|GetWorldLocation _skeletalmeshcomponent)))) true false))

(fn SetSimulateAll
  (bind _skeletalmeshcomponent (Variables|SkeletalMeshActor|GetSkeletalMeshComponent))
  (Class|SkeletalMeshComponent|SetAllBodiesBelowSimulatePhysics (Variables|SkeletalMeshActor|GetSkeletalMeshComponent) (Utilities|Name|MakeLiteralName (.BoneName (Class|SkeletalMeshComponent|GetClosestPointonPhysicsAsset _skeletalmeshcomponent (Transformation|GetWorldLocation _skeletalmeshcomponent)))) true true))