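; BP_Spawner is a sushi shop spawner actor that periodically creates boats carrying customer orders.
; On BeginPlay it starts a looping timer that spawns a BP_Boat at its own transform until a boat cap is reached.
; Each boat gets one requirement with a random sushi name and amount, plus the ScoreDisplay widget taken from the Scoreboard.
; The boat count only increments here.
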(event Custom|Spawn%20Boat
  (if (< (Variables|Default|GetNumOfBoats) (Variables|Default|GetMaxBoats))
    (bind _asscore_display (Utilities|Casting|CastToScoreDisplay (UserInterface|GetUserWidgetObject (Variables|Default|GetScoreboard))))
    (Game|SpawnActorfromClass "/Game/SushiShop/BluePrints/New/Boat/BP_Boat.BP_Boat_C" (Transformation|GetActorTransform) "Undefined" 0 (Utilities|Array|MakeArray (Utilities|Struct|MakeBP_Requirement (Math|Random|RandomIntegerinRange 1 6) (Utilities|Array|Get(acopy) (Variables|Default|GetSushi) (Math|Random|RandomIntegerinRange 0 2)))) _asscore_display 0)
    (Math|Integer|IncrementInt (Variables|Default|GetNumOfBoats))))

(event EventBeginPlay
  (Utilities|Time|SetTimerbyEvent (delegate Custom|Spawn%20Boat) (Variables|Default|GetSpawnTime) true))

(fn ConstructionScript)