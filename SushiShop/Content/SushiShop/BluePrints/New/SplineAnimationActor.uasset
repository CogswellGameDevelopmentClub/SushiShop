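; SplineAnimationActor is an actor that moves its Cube1 component along its Spline, apparently as a boat animation given the timeline's name.
; BoatTimeline starts on BeginPlay, and its Main track is multiplied by the spline length to give a distance along the path.
; Each timeline update sets the cube's world location and rotation from the spline at that distance, keeping its current scale.
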(event EventBeginPlay
  (bind _spline (Variables|Default|GetSpline))
  (bind _main (Timeline|Boat%20Timeline PlayFromStart)
    (:Update
      (Transformation|SetWorldTransform (Variables|Default|GetCube1) (Math|Transform|MakeTransform (Spline|GetLocationatDistanceAlongSpline _spline (* _main (Spline|GetSplineLength _spline)) "World") (Spline|GetRotationatDistanceAlongSpline _spline (* _main (Spline|GetSplineLength _spline)) "World") (Transformation|GetWorldScale (Variables|Default|GetCube1))) false false))))

(event Collision|EventActorBeginOverlap
  (params (OtherActor :type Actor%20Object%20Reference)))

(event EventTick
  (params (DeltaSeconds :type Float%20%28single-precision%29)))

(fn ConstructionScript)