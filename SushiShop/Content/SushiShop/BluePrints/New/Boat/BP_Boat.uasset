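; Sushi shop boat that rides along a spline and tracks whether the ingredients placed on it fulfil its order.
; A timeline started on BeginPlay drives the mesh's position and rotation along the spline.
; Trigger overlaps identify tuna, salmon, unagi or rice through a chain of casts, then adjust ingredient counts.
; Each change rechecks completion by exact name-and-amount match and refreshes the child-actor order menu.
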(event OnComponentBeginOverlap(Trigger)
  (params (OverlappedComponent :type Primitive%20Component%20Object%20Reference) (OtherActor :type Actor%20Object%20Reference) (OtherComp :type Primitive%20Component%20Object%20Reference) (OtherBodyIndex :type Integer) (bFromSweep :type Boolean) (SweepResult :type Hit%20Result%20Structure%20%28by%20ref%29))
  ;[0.09705 1 0.8298] System to detect objects on the boat based on class
  (Variables|Default|SetNameInBoat "NaF")
  (bind _nameinboat (CallFunction|CastingClass OtherActor))
  (if (Utilities|Enum|NotEqual(Enum) _nameinboat "NaF")
    (CallFunction|AddIngredient _nameinboat)))

(event OnComponentEndOverlap(Trigger)
  (params (OverlappedComponent :type Primitive%20Component%20Object%20Reference) (OtherActor :type Actor%20Object%20Reference) (OtherComp :type Primitive%20Component%20Object%20Reference) (OtherBodyIndex :type Integer))
  ;[0.09705 1 0.8298] System to detect objects on the boat based on class
  (Variables|Default|SetNameInBoat "NaF")
  (bind _nameinboat (CallFunction|CastingClass OtherActor))
  (if (Utilities|Enum|NotEqual(Enum) _nameinboat "NaF")
    (CallFunction|RemoveIngredient _nameinboat)))

(event EventBeginPlay
  ;[0.7054 0 1] Spline Transform system to move boats.
  (CallFunction|CreateMenu)
  (bind _main (|Timeline)
    (:Update
      (CallFunction|FSplineTransform _main))))

(fn ConstructionScript)

(fn UpdateWidget
  (Default|UpdateItemList (Variables|Default|GetOrder%20Menu) (Variables|Default|GetCurrent%20Ingredients)))

(fn UpdateCompleteStatus
  (for _array_element (Variables|OrderInfo|GetOrder%20Reqs)
    (if (not (Utilities|Array|ContainsItem (Variables|Default|GetCurrent%20Ingredients) _array_element))
      ;[0 0 0] If any req isn't met, it's not done
      (Variables|OrderInfo|SetOrder%20Complete false)
      (return)))
  ;[0 0 0] If we made it thru, it's complete
  (Variables|OrderInfo|SetOrder%20Complete true))

(fn RemoveIngredient
  (params (Name :type String))
  (for (_array_element _array_index) (Variables|Default|GetCurrent%20Ingredients)
    ;[1 1 1] If we can find it on the list
    (if (Utilities|Enum|Equal(Enum) (.Name (Utilities|Struct|BreakBP_Requirement _array_element)) Name)
      (if (> (.Amount (Utilities|Struct|BreakBP_Requirement _array_element)) 1)
        ;[1 1 1] Decrease the count by 1
        (Utilities|Array|SetArrayElem (Variables|Default|GetCurrent%20Ingredients) _array_index (Utilities|Struct|MakeBP_Requirement (- (.Amount (Utilities|Struct|BreakBP_Requirement _array_element)) 1) (.Name (Utilities|Struct|BreakBP_Requirement _array_element))))
        (else
          ;[1 1 1] If you can't decrement, remove entirely
          (Utilities|Array|RemoveIndex (Variables|Default|GetCurrent%20Ingredients) _array_index)))
      (CallFunction|UpdateCompleteStatus)
      (CallFunction|UpdateWidget)
      (return))))

(fn AddIngredient
  (params (Name :type String))
  (for (_array_element _array_index) (Variables|Default|GetCurrent%20Ingredients)
    ;[1 1 1] If we can find it on the list
    (if (Utilities|Enum|Equal(Enum) (.Name (Utilities|Struct|BreakBP_Requirement _array_element)) Name)
      ;[1 1 1] Increase the count by 1
      (Utilities|Array|SetArrayElem (Variables|Default|GetCurrent%20Ingredients) _array_index (Utilities|Struct|MakeBP_Requirement (+ (.Amount (Utilities|Struct|BreakBP_Requirement _array_element)) 1) (.Name (Utilities|Struct|BreakBP_Requirement _array_element))))
      (CallFunction|UpdateCompleteStatus)
      (CallFunction|UpdateWidget)
      (return)))
  ;[1 1 1] If not found, add to list
  (Utilities|Array|Add (Variables|Default|GetCurrent%20Ingredients) (Utilities|Struct|MakeBP_Requirement 1 Name))
  (CallFunction|UpdateCompleteStatus)
  (CallFunction|UpdateWidget)
  (return))

(fn CreateMenu
  (bind _asbp_order_menu (Utilities|Casting|CastToBP_OrderMenu (Variables|/Script/Engine.ChildActorComponent|GetChildActor (Variables|Default|GetMenu)))
    (:then
      (Variables|Default|SetOrder%20Menu _asbp_order_menu)
      (for _array_element (Variables|OrderInfo|GetOrder%20Reqs)
        (Default|AddItem (Variables|Default|GetOrder%20Menu) _array_element)))
    (:CastFailed
      (Development|PrintString "Error: Boat menu not a menu!" true true "(R=1.000000,G=0.009182,B=0.000000,A=1.000000)"))))

(fn CastingClass
  (params (Object :type Object%20Object%20Reference))
  ;[0 0.09693 1] Add Function here to allow the system to cast to each object
  (CallFunction|FTunaCast Object)
  (CallFunction|FSalmonCast Object)
  (CallFunction|FUnagiCast Object)
  (CallFunction|FRiceCast Object)
  (return (Variables|Default|GetNameInBoat)))

(fn FTunaCast
  (params (Object :type Object%20Object%20Reference))
  (bind _aspc_tuna (Utilities|Casting|CastToPC_Tuna Object)
    (:then
      (Variables|Default|SetNameInBoat (Variables|/Game/SushiShop/BluePrints/New/ItemHandling/BP_Physics.BP_Physics_C|GetName _aspc_tuna)))
    (:CastFailed
      (Variables|Default|SetNameInBoat (Variables|Default|GetNameInBoat)))))

(fn FSalmonCast
  (params (Object :type Object%20Object%20Reference))
  (bind _aspc_salmon (Utilities|Casting|CastToPC_Salmon Object)
    (:then
      (Variables|Default|SetNameInBoat (Variables|/Game/SushiShop/BluePrints/New/ItemHandling/BP_Physics.BP_Physics_C|GetName _aspc_salmon)))
    (:CastFailed
      (Variables|Default|SetNameInBoat (Variables|Default|GetNameInBoat)))))

(fn FUnagiCast
  (params (Object :type Object%20Object%20Reference))
  (bind _aspc_unagi (Utilities|Casting|CastToPC_Unagi Object)
    (:then
      (Variables|Default|SetNameInBoat (Variables|/Game/SushiShop/BluePrints/New/ItemHandling/BP_Physics.BP_Physics_C|GetName _aspc_unagi)))
    (:CastFailed
      (Variables|Default|SetNameInBoat (Variables|Default|GetNameInBoat)))))

(fn FRiceCast
  (params (Object :type Object%20Object%20Reference))
  (bind _aspc_rice (Utilities|Casting|CastToPC_Rice Object)
    (:then
      (Variables|Default|SetNameInBoat (Variables|/Game/SushiShop/BluePrints/New/ItemHandling/BP_Physics.BP_Physics_C|GetName _aspc_rice)))
    (:CastFailed
      (Variables|Default|SetNameInBoat (Variables|Default|GetNameInBoat)))))

(fn FSplineTransform
  (params (A :type Float%20%28single-precision%29))
  (bind _spline (Variables|Default|GetSpline))
  (bind _spline_2 (Variables|Default|GetSpline))
  (bind _returnvalue (Spline|GetSplineLength _spline_2))
  (bind _returnvalue_2 (* A _returnvalue))
  (Transformation|SetWorldTransform (Variables|Default|GetStaticMesh) (Math|Transform|MakeTransform (Spline|GetLocationatDistanceAlongSpline _spline _returnvalue_2 "World") (Spline|GetRotationatDistanceAlongSpline _spline _returnvalue_2 "World") (Transformation|GetWorldScale (Variables|Default|GetStaticMesh))) false false))