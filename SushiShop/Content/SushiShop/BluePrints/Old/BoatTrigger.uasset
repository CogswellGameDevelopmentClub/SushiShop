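; BoatTrigger is an overlap trigger that tracks which actors are on the boat for the sushi shop's order checklist.
; On BeginPlay it looks up the first Display_Order widget and stores it as the checklist reference.
; Begin and end overlaps add or remove actors in BoatArray, notify the widget's CompletionStatus to update check marks, and print the array for debugging.
; AddToBoatArray is an empty stub.
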(event EventBeginPlay
  ;[1 0 0.9175] Cast to the Widget Class and get all widgets of that class as an object reference so the Completion status function has a target.
  (bind _asdisplay_order (Utilities|Casting|CastToDisplay_OrderClass "/Game/SushiShop/BluePrints/Old/Display_Order.Display_Order_C")
    (:then
      (bind _foundwidgets (Widget|GetAllWidgetsOfClass _asdisplay_order false))
      (if (Utilities|Array|IsValidIndex _foundwidgets)
        (Variables|Default|SetCheck%20List%20Reference (Utilities|Array|Get(acopy) _foundwidgets))))
    (:CastFailed
      (Development|PrintString "Cast to Widget Class failed" true true "(R=0.000000,G=0.660000,B=1.000000,A=1.000000)" 1e+01))))

(event Collision|EventActorBeginOverlap
  (params (OtherActor :type Actor%20Object%20Reference))
  ;[1 0.6039 0.195] On Overlap, add the offending actor to a list, On End overlap, remove the scum from the list
  (Utilities|Array|Add (Variables|Default|GetBoat%20Array) OtherActor)
  ;;[0.1008 0 1] This sends the offending object to the completion Status function where it checks to see if all needed objects are on the boat, if they are, it changes the check state of the releated check mark
  (Default|CompletionStatus (Variables|Default|GetCheck%20List%20Reference) OtherActor true)
  (for _array_element (Variables|Default|GetBoat%20Array)
    (Development|PrintString (Utilities|GetDisplayName _array_element) true true "(R=1.000000,G=0.259897,B=0.786832,A=1.000000)" 1e+01)))

(event EventTick
  (params (DeltaSeconds :type Float%20%28single-precision%29)))

(event Collision|EventActorEndOverlap
  (params (OtherActor :type Actor%20Object%20Reference))
  (bind _boat_array (Variables|Default|GetBoat%20Array))
  ;[1 0.6039 0.195] On Overlap, add the offending actor to a list, On End overlap, remove the scum from the list
  (Utilities|Array|RemoveIndex _boat_array (Utilities|Array|FindItem _boat_array OtherActor))
  ;;[0.1008 0 1] This sends the offending object to the completion Status function where it checks to see if all needed objects are on the boat, if they are, it changes the check state of the releated check mark
  (Default|CompletionStatus (Variables|Default|GetCheck%20List%20Reference) OtherActor false)
  (for _array_element (Variables|Default|GetBoat%20Array)
    (Development|PrintString (Utilities|GetDisplayName _array_element) true true "(R=0.099006,G=0.445833,B=0.056897,A=1.000000)" 1e+01)))

(fn ConstructionScript)

(fn AddtoBoatArray)