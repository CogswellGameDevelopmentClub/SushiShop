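; BP_Boat is a sushi shop order boat that tracks which ingredients sit in its trigger and whether they satisfy its order.
; Overlap begin and end add or remove BPP_Ingredient names in a counted list, then recheck completion and refresh the menu.
; The child-actor BP_OrderMenu is filled from the order requirements at BeginPlay.
; Completion matches whole requirement structs, so amounts must be exact, while unrequested extras are ignored.
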(event OnComponentBeginOverlap(Trigger)
  (params (OverlappedComponent :type Primitive%20Component%20Object%20Reference) (OtherActor :type Actor%20Object%20Reference) (OtherComp :type Primitive%20Component%20Object%20Reference) (OtherBodyIndex :type Integer) (bFromSweep :type Boolean) (SweepResult :type Hit%20Result%20Structure%20%28by%20ref%29))
  (bind _asbpp_ingredient (Utilities|Casting|CastToBPP_Ingredient OtherActor))
  (CallFunction|AddIngredient (Variables|/Game/SushiShop/BluePrints/Scott_Remake/BPP_Ingredient.BPP_Ingredient_C|GetName _asbpp_ingredient)))

(event OnComponentEndOverlap(Trigger)
  (params (OverlappedComponent :type Primitive%20Component%20Object%20Reference) (OtherActor :type Actor%20Object%20Reference) (OtherComp :type Primitive%20Component%20Object%20Reference) (OtherBodyIndex :type Integer))
  (bind _asbpp_ingredient (Utilities|Casting|CastToBPP_Ingredient OtherActor))
  (CallFunction|RemoveIngredient (Variables|/Game/SushiShop/BluePrints/Scott_Remake/BPP_Ingredient.BPP_Ingredient_C|GetName _asbpp_ingredient)))

(event EventBeginPlay
  (CallFunction|CreateMenu))

(fn ConstructionScript)

(fn UpdateWidget
  (Default|UpdateItemList (Variables|Default|GetOrder%20Menu) (Variables|Default|GetCurrent%20Ingredients)))

(fn UpdateCompleteStatus
  (for _array_element (Variables|OrderInfo|GetOrder%20Reqs)
    (if (not (Utilities|Array|ContainsItem (Variables|Default|GetCurrent%20Ingredients) _array_element))
      ;[1 1 1] If any req isn't met, it's not done
      (Variables|OrderInfo|SetOrder%20Complete false)
      (return)))
  ;[1 1 1] If we made it thru, it's complete
  (Variables|OrderInfo|SetOrder%20Complete true))

(fn RemoveIngredient
  (params (Name :type String))
  (for (_array_element _array_index) (Variables|Default|GetCurrent%20Ingredients)
    ;[1 1 1] If we can find it on the list
    (if (Utilities|Enum|Equal(Enum) (.Name (Utilities|Struct|BreakBP_Requirement _array_element)) Name)
      (if (> (.Amount (Utilities|Struct|BreakBP_Requirement _array_element)) 1)
        ;[1 1 1] Decrease the count by 1
        (Utilities|Array|SetArrayElem (Variables|Default|GetCurrent%20Ingredients) _array_index (Utilities|Struct|MakeBP_Requirement (- (.Amount (Utilities|Struct|BreakBP_Requirement _array_element)) 1) (.Name (Utilities|Struct|BreakBP_Requirement _array_element))))
        (else
          ;[1 1 1] If you can't decrement, remove entirely
          (Utilities|Array|RemoveIndex (Variables|Default|GetCurrent%20Ingredients) _array_index)))
      (CallFunction|UpdateCompleteStatus)
      (CallFunction|UpdateWidget)
      (return))))

(fn AddIngredient
  (params (Name :type String))
  (for (_array_element _array_index) (Variables|Default|GetCurrent%20Ingredients)
    ;[1 1 1] If we can find it on the list
    (if (Utilities|Enum|Equal(Enum) (.Name (Utilities|Struct|BreakBP_Requirement _array_element)) Name)
      ;[1 1 1] Increase the count by 1
      (Utilities|Array|SetArrayElem (Variables|Default|GetCurrent%20Ingredients) _array_index (Utilities|Struct|MakeBP_Requirement (+ (.Amount (Utilities|Struct|BreakBP_Requirement _array_element)) 1) (.Name (Utilities|Struct|BreakBP_Requirement _array_element))))
      (CallFunction|UpdateCompleteStatus)
      (CallFunction|UpdateWidget)
      (return)))
  ;[1 1 1] If not found, add to list
  (Utilities|Array|Add (Variables|Default|GetCurrent%20Ingredients) (Utilities|Struct|MakeBP_Requirement 1 Name))
  (CallFunction|UpdateCompleteStatus)
  (CallFunction|UpdateWidget)
  (return))

(fn CreateMenu
  (bind _asbp_order_menu (Utilities|Casting|CastToBP_OrderMenu (Variables|/Script/Engine.ChildActorComponent|GetChildActor (Variables|Default|GetMenu)))
    (:then
      (Variables|Default|SetOrder%20Menu _asbp_order_menu)
      (for _array_element (Variables|OrderInfo|GetOrder%20Reqs)
        (Default|AddItem (Variables|Default|GetOrder%20Menu) _array_element)))
    (:CastFailed
      (Development|PrintString "Error: Boat menu not a menu!" true true "(R=1.000000,G=0.009182,B=0.000000,A=1.000000)"))))