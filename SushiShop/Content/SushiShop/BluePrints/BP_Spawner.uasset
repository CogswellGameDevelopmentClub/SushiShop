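; BP_Spawner periodically spawns BP_Boat actors at its own transform for the sushi shop game.
; A looping timer started at BeginPlay fires SpawnBoat, which spawns only while the boat count is below MaxBoats.
; Each boat receives one randomized order requirement: an amount and a name picked from the first two Sushi array entries.
; The count only increments in this Blueprint.
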(event Custom|Spawn%20Boat
  (if (< (Variables|Default|GetNumOfBoats) (Variables|Default|GetMaxBoats))
    (Game|SpawnActorfromClass "/Game/SushiShop/BluePrints/Boat/BP_Boat.BP_Boat_C" (Transformation|GetActorTransform) "Undefined" 0 (Utilities|Array|MakeArray (Utilities|Struct|MakeBP_Requirement (Math|Random|RandomIntegerinRange 1 6) (Utilities|Array|Get(acopy) (Variables|Default|GetSushi) (Math|Random|RandomIntegerinRange 0 1)))) 0)
    (Math|Integer|IncrementInt (Variables|Default|GetNumOfBoats))))

(event EventBeginPlay
  (Utilities|Time|SetTimerbyEvent (delegate Custom|Spawn%20Boat) (Variables|Default|GetSpawnTime) true))

(fn ConstructionScript)