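; A physics-driven salmon slice actor in the sushi shop that can be picked up and dropped through a pickup interface.
; Pickup stops mesh simulation, attaches the root to the given component in world space, then re-enables physics only on bones below the root joint, leaving the rest of the slice physical while held.
; Drop restores simulation on the whole skeletal mesh, root bone included, and detaches the actor in place.
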(event EventBeginPlay)

(event Collision|EventActorBeginOverlap
  (params (OtherActor :type Actor%20Object%20Reference)))

(event EventPickup
  (params (Attach%20TO :type Scene%20Component%20Object%20Reference))
  ;[1 1 1] Open Class Settings and add the Pickup Actor Interface
  (Physics|SetSimulatePhysics (Variables|SkeletalMeshActor|GetSkeletalMeshComponent) false)
  (Transformation|AttachComponentToComponent (VehicleSound|GetRootComponent) Attach%20TO "None" "KeepWorld" "KeepWorld" "KeepWorld" false)
  (Class|SkeletalMeshComponent|SetAllBodiesBelowSimulatePhysics (Variables|SkeletalMeshActor|GetSkeletalMeshComponent) (Utilities|Name|MakeLiteralName "SalmonSliceJoint_Root") true false))

(event EventDrop
  ;[1 1 1] Open Class Settings and add the Pickup Actor Interface
  (Class|SkeletalMeshComponent|SetAllBodiesBelowSimulatePhysics (Variables|SkeletalMeshActor|GetSkeletalMeshComponent) (Utilities|Name|MakeLiteralName "SalmonSliceJoint_Root") true true)
  (Physics|SetSimulatePhysics (Variables|SkeletalMeshActor|GetSkeletalMeshComponent) true)
  (Transformation|DetachFromActor "KeepWorld" "KeepWorld" "KeepWorld"))

(event EventTick
  (params (DeltaSeconds :type Float%20%28single-precision%29)))

(fn ConstructionScript)