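; Motion-controller pickup for a mesh, held by attachment, physics handle or a mixed mode set by GrabMethod.
; For the latter two, Tick swaps to the physics handle when the mesh overlaps objects other than motion controllers.
; Once clear, recent hits let it lerp to the stored hand offset and reattach, using DoOnce gates.
; Those modes also auto-drop the item if it strays too far from the controller.
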(event OnComponentHit(StaticMesh)
  (params (HitComponent :type Primitive%20Component%20Object%20Reference) (OtherActor :type Actor%20Object%20Reference) (OtherComp :type Primitive%20Component%20Object%20Reference) (NormalImpulse :type Vector :default "0, 0, 0") (Hit :type Hit%20Result%20Structure%20%28by%20ref%29))
  (bind _is_hit (CallFunction|IsValidHit OtherActor))
  (if _is_hit
    (Variables|Default|SetHit%20Time (Utilities|Time|GetGameTimeinSeconds))))

(event Custom|OpenDoOnceGates
  (Utilities|FlowControl|Sequence
    (:then_0
      (Utilities|FlowControl|DoOnce false) ; enters at Reset
    )
    (:then_1
      (Utilities|FlowControl|DoOnce false) ; enters at Reset
    )))

(event EventBeginPlay
  (bind _outactors (Actor|GetAllActorsOfClass "/Game/VirtualRealityBP/Blueprints/BP_MotionController.BP_MotionController_C"))
  (Variables|Default|SetActors%20To%20Ignore _outactors))

(event Collision|EventActorBeginOverlap
  (params (OtherActor :type Actor%20Object%20Reference)))

(event EventTick
  (params (DeltaSeconds :type Float%20%28single-precision%29))
  (bind _staticmesh (Variables|Default|GetStaticMesh))
  (switch Utilities|FlowControl|Switch|SwitchonEGrabMethod (Variables|Default|GetGrabMethod)
    (:NewEnumerator1
      (CallFunction|DropifLostConnection))
    (:NewEnumerator2
      (CallFunction|DropifLostConnection)))
  (if (Utilities|IsValid (Variables|Default|GetMC))
    (bind _returnvalue (Class|KismetSystemLibrary|ComponentOverlapComponents _staticmesh (Transformation|GetWorldTransform _staticmesh) (Utilities|Array|MakeArray "ObjectTypeQuery1" "ObjectTypeQuery2" "ObjectTypeQuery4" "ObjectTypeQuery7") 0 (Variables|Default|GetActors%20To%20Ignore)))
    (if _returnvalue
      (Utilities|FlowControl|DoOnce false :!label _label
        (:Completed
          (CallFunction|DropAttachto)
          (CallFunction|PHAttach)
          (goto _label_2 Reset)))
      (elif (< (- (Utilities|Time|GetGameTimeinSeconds) (Variables|Default|GetHit%20Time)) 0.1)
        (if (> (Variables|Default|GetLocationAlpha) 1.0)
          (Utilities|FlowControl|DoOnce false :!label _label_2
            (:Completed
              (CallFunction|PHDrop)
              (CallFunction|GrabAttachto)
              (goto _label Reset)))
          (else
            (Variables|Default|SetLocationAlpha (+ (Variables|Default|GetLocationAlpha) (* (Utilities|Time|GetWorldDeltaSeconds) 1e+01)))
            (Transformation|SetWorldLocationAndRotation (Variables|Default|GetStaticMesh) (.location (Math|Transform|Lerp(Transform) (Transformation|GetWorldTransform (Variables|Default|GetStaticMesh)) (Utilities|GetWorldPickupTransform) (Variables|Default|GetLocationAlpha))) (.rotation (Math|Transform|Lerp(Transform) (Transformation|GetWorldTransform (Variables|Default|GetStaticMesh)) (Utilities|GetWorldPickupTransform) (Variables|Default|GetLocationAlpha))) false false)))))))

(event EventPickup
  (params (MC :type Scene%20Component%20Object%20Reference) (PH :type Physics%20Handle%20Component%20Object%20Reference))
  (Utilities|FlowControl|Sequence
    (:then_0
      (Utilities|IsValid (Variables|Default|GetMC)
        (:Is%20Valid
          (CallFunction|Drop))))
    (:then_1
      (Variables|Default|SetMC MC)
      (Variables|Default|SetPH PH))
    (:then_2
      (switch Utilities|FlowControl|Switch|SwitchonEGrabMethod (Variables|Default|GetGrabMethod)
        (:NewEnumerator0
          (CallFunction|GrabAttachto))
        (:NewEnumerator1
          (CallFunction|PHAttach))
        (:NewEnumerator2
          (CallFunction|GrabMixedMode))))))

(event EventDrop
  (Utilities|FlowControl|Sequence
    (:then_0
      (switch Utilities|FlowControl|Switch|SwitchonEGrabMethod (Variables|Default|GetGrabMethod)
        (:NewEnumerator0
          (CallFunction|DropAttachto))
        (:NewEnumerator1
          (CallFunction|PHDrop))
        (:NewEnumerator2
          (CallFunction|DropMixedMode))))
    (:then_1
      (Variables|Default|SetMC 0)
      (Variables|Default|SetPH 0))))

(fn ConstructionScript)

(fn GrabAttachto
  (bind _transform (Utilities|GetWorldPickupTransform))
  (Collision|SetCollisionObjectType (Variables|Default|GetStaticMesh) "ECC_GameTraceChannel1")
  (Physics|SetEnableGravity (Variables|Default|GetStaticMesh) false)
  (Physics|SetSimulatePhysics (Variables|Default|GetStaticMesh) false)
  (if (Variables|Default|GetIsGrabbed)
    (Transformation|SetWorldLocationAndRotation (Variables|Default|GetStaticMesh) (.location _transform) (.rotation _transform) false false))
  (Transformation|AttachComponentToComponent (VehicleSound|GetRootComponent) (Variables|Default|GetMC) "None" "KeepWorld" "KeepWorld" "KeepWorld" true)
  (if (not (Variables|Default|GetIsGrabbed))
    (Variables|Default|SetRelativePickupOffset (Utilities|GetRelativePickupTransform))))

(fn PHAttach
  (bind _mc (Variables|Default|GetMC))
  (bind _returnvalue (Transformation|GetWorldTransform _mc))
  (Physics|Components|PhysicsHandle|GrabComponentatLocationwithRotation (Variables|Default|GetPH) (Variables|Default|GetStaticMesh) "None" (.location _returnvalue) (.rotation _returnvalue))
  (Physics|SetEnableGravity (Variables|Default|GetStaticMesh) false)
  (Physics|SetSimulatePhysics (Variables|Default|GetStaticMesh) true)
  (Collision|SetCollisionObjectType (Variables|Default|GetStaticMesh) "ECC_PhysicsBody")
  (Variables|Default|SetLocationAlpha 0.0))

(fn DropAttachto
  (Physics|SetSimulatePhysics (Variables|Default|GetStaticMesh) true)
  (Transformation|DetachFromActor "KeepWorld" "KeepWorld" "KeepWorld"))

(fn PHDrop
  (Physics|Components|PhysicsHandle|ReleaseComponent (Variables|Default|GetPH))
  (Physics|SetEnableGravity (Variables|Default|GetStaticMesh) true))

(fn GrabMixedMode
  (Collision|SetCollisionResponsetoChannel (Variables|Default|GetStaticMesh) "ECC_Pawn" "ECR_Ignore")
  (CallFunction|GrabAttachto)
  (Variables|Default|SetIsGrabbed true)
  (CallFunction|OpenDoOnceGates))

(fn DropMixedMode
  (Variables|Default|SetIsGrabbed false)
  (CallFunction|DropAttachto)
  (CallFunction|PHDrop)
  (Collision|SetCollisionObjectType (Variables|Default|GetStaticMesh) "ECC_PhysicsBody")
  (Collision|SetCollisionResponsetoChannel (Variables|Default|GetStaticMesh) "ECC_Pawn" "ECR_Block")
  (Variables|Default|SetLocationAlpha 0.0))

(fn IsValidHit
  (params (Actor :type Actor%20Object%20Reference))
  (LocalVariables|SetHitValid true)
  (for _array_element (Variables|Default|GetActors%20To%20Ignore)
    (if (== _array_element Actor)
      (LocalVariables|SetHitValid false)))
  (return (LocalVariables|GetHitValid)))

(fn DropifLostConnection
  (Utilities|IsValid (Variables|Default|GetMC)
    (:Is%20Valid
      (if (> (Math|Vector|VectorLength (- (Transformation|GetWorldLocation (Variables|Default|GetStaticMesh)) (Transformation|GetWorldLocation (Variables|Default|GetMC)))) 3e+01)
        (CallFunction|Drop)
        (return)))
    (:Is%20Not%20Valid
      (return))))

(fn IsHeldbyMe
  (params (MC :type Motion%20Controller%20Component%20Object%20Reference))
  (return (== MC (Variables|Default|GetMC))))